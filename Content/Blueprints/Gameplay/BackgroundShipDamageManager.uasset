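; Manager actor that applies periodic background damage to the player's ship for as long as it is in play.
; A one-shot timer re-arms itself at a random interval within a frequency range, even while damage is disabled.
; When enabled, each tick spawns an explosion at a fixed distance in a random direction from the player, then deals slight ship damage through OnlyOneGameMode.
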(event Custom|ScheduleBackgroundDamage
  (bind _returnvalue (Utilities|Time|SetTimerbyEvent (delegate Custom|DoBackgroundDamage) (Math|Random|RandomFloatinRange (Variables|Default|GetMinFrequency) (Variables|Default|GetMaxFrequency))))
  (Variables|Default|SetTimerHandle _returnvalue))

(event Custom|DoBackgroundDamage
  (Utilities|FlowControl|Sequence
    (:then_0
      (if (Variables|Default|GetBackgroundDamageEnabled)
        (CallFunction|SpawnExplosionAroundPlayer)
        (bind _asonly_one_game_mode (Utilities|Casting|CastToOnlyOneGameMode (Game|GetGameMode)))
        (Default|TakeShipDamage _asonly_one_game_mode 0.05)))
    (:then_1
      (CallFunction|ScheduleBackgroundDamage))))

(event EventBeginPlay
  (CallFunction|ScheduleBackgroundDamage))

(fn ConstructionScript)

(fn SpawnExplosionAroundPlayer
  (bind _returnvalue (Game|GetPlayerCharacter 0))
  (Utilities|IsValid _returnvalue
    (:Is%20Valid
      (Game|SpawnActorfromClass "/Game/Blueprints/Gameplay/BackgroundExplosion.BackgroundExplosion_C" (Math|Transform|MakeTransform (+ (Transformation|GetActorLocation _returnvalue) (* (Math|Random|RandomUnitVector) (Variables|Default|GetExplosionDistanceFromPlayer)))) "AlwaysSpawn" 0 0))))