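; Groups a set of child-actor buttons, apparently for a player room, behind a single pressed event.
; On BeginPlay it collects ButtonBP instances from its ChildActorComponents into a Buttons array, then binds each one's OnButtonPressed to a shared handler.
; That handler rebroadcasts the actor's own OnButtonPressed dispatcher without passing on which button was pressed.
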(event Custom|ButtonPressed
  (Utilities|FlowControl|Sequence
    (:then_1
      (Default|CallOnButtonPressed))))

(event EventBeginPlay
  (Utilities|FlowControl|Sequence
    (:then_0
      (for _array_element (Actor|GetComponentsByClass "/Script/Engine.ChildActorComponent")
        (bind _asbutton_bp (Utilities|Casting|CastToButtonBP (Variables|/Script/Engine.ChildActorComponent|GetChildActor _array_element)))
        (Utilities|Array|Add (Variables|Default|GetButtons) _asbutton_bp)))
    (:then_1
      (for _array_element_2 (Variables|Default|GetButtons)
        (EventDispatchers|BindEventtoOnButtonPressed _array_element_2 (delegate Custom|ButtonPressed))))))

(fn ConstructionScript)