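; Blueprint function library that gives gameplay code access to the managers for the ship's rooms and elevator.
; Each getter casts the current game mode to OnlyOneGameMode and returns one of its manager references: Navigation, Tactical, Engineering, Elevator or Crew Quarters.
; A failed cast returns an empty result.
; Because it reads the game mode, these lookups only resolve where that game mode exists.
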(fn GetNavigationRoomManager
  (params (WorldContextObject :type Object%20Object%20Reference))
  (bind _asonly_one_game_mode (Utilities|Casting|CastToOnlyOneGameMode (Game|GetGameMode WorldContextObject))
    (:then
      (return (Variables|/Game/Blueprints/OnlyOneGameMode.OnlyOneGameMode_C|GetNavigationRoomManager _asonly_one_game_mode)))
    (:CastFailed
      (return 0))))

(fn GetTacticalRoomManager
  (params (WorldContextObject :type Object%20Object%20Reference))
  (bind _asonly_one_game_mode (Utilities|Casting|CastToOnlyOneGameMode (Game|GetGameMode WorldContextObject))
    (:then
      (return (Variables|/Game/Blueprints/OnlyOneGameMode.OnlyOneGameMode_C|GetTacticalRoomManager _asonly_one_game_mode)))
    (:CastFailed
      (return 0))))

(fn GetEngineeringRoomManager
  (params (WorldContextObject :type Object%20Object%20Reference))
  (bind _asonly_one_game_mode (Utilities|Casting|CastToOnlyOneGameMode (Game|GetGameMode WorldContextObject))
    (:then
      (return (Variables|/Game/Blueprints/OnlyOneGameMode.OnlyOneGameMode_C|GetEngineeringRoomManager _asonly_one_game_mode)))
    (:CastFailed
      (return 0))))

(fn GetElevatorManager
  (params (WorldContextObject :type Object%20Object%20Reference))
  (bind _asonly_one_game_mode (Utilities|Casting|CastToOnlyOneGameMode (Game|GetGameMode WorldContextObject))
    (:then
      (return (Variables|/Game/Blueprints/OnlyOneGameMode.OnlyOneGameMode_C|GetElevatorManager _asonly_one_game_mode)))
    (:CastFailed
      (return 0))))

(fn GetCrewQuartersManager
  (params (WorldContextObject :type Object%20Object%20Reference))
  (bind _asonly_one_game_mode (Utilities|Casting|CastToOnlyOneGameMode (Game|GetGameMode WorldContextObject))
    (:then
      (return (Variables|/Game/Blueprints/OnlyOneGameMode.OnlyOneGameMode_C|GetCrewQuartersManager _asonly_one_game_mode)))
    (:CastFailed
      (return 0))))