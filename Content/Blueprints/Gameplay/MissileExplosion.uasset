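; Missile explosion effect actor that stages the audio and player feedback for a missile strike.
; On BeginPlay it starts fire and Doppler sounds, then after a short delay plays the explosion sound with a large world camera shake.
; The shake uses a huge radius with zero falloff and orients toward the actor.
; The blast also briefly slows the player character's look and movement input through PlayerCharacterBP.
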(event EventBeginPlay
  (Audio|Components|Audio|Play (Variables|Default|GetFireSound) 0.0)
  (Audio|Components|Audio|Play (Variables|Default|GetDoppler) 0.0)
  (Utilities|FlowControl|Delay 1.3)
  (Camera|PlayWorldCameraShake "/Game/Blueprints/Gameplay/ExplosionCameraShake_Large.ExplosionCameraShake_Large_C" (Transformation|GetActorLocation) 0.0 1e+06 0.0 true)
  (Audio|Components|Audio|Play (Variables|Default|GetExplosionSound) 0.0)
  (bind _asplayer_character_bp (Utilities|Casting|CastToPlayerCharacterBP (Game|GetPlayerCharacter 0)))
  (Default|SlowInputforDuration _asplayer_character_bp 0.3 0.3 1.0))

(fn ConstructionScript)