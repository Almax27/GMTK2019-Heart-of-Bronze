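; Tactical room manager that oversees a set of cabinets and doors, rewarding successful cabinet results with gun charge.
; On BeginPlay it binds to each valid cabinet's result event and, on success, adds charge through OnlyOneGameMode.
; It exposes functions to activate and return a random inactive cabinet and to unlock all its doors; neither is called within this Blueprint.
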(event Custom|CabinetResult
  (params (result :type Cabinet%20Result%20Structure))
  (switch name (.result (Utilities|Struct|BreakCabinetResult result))
    (:Success
      (bind _asonly_one_game_mode (Utilities|Casting|CastToOnlyOneGameMode (Game|GetGameMode)))
      (Default|AddGunCharge _asonly_one_game_mode 0.1))))

(event EventBeginPlay
  (for _array_element (Variables|Default|GetCabinets)
    (Utilities|IsValid _array_element
      (:Is%20Valid
        (EventDispatchers|BindEventtoOnCabinetResult _array_element (delegate Custom|CabinetResult))))))

(fn ConstructionScript)

(fn ActivateRandomCabinet
  (LocalVariables|SetInactiveCabinets (CallFunction|GetInactiveCabinets))
  (bind _output_get (LocalVariables|SetRandomIndex (Math|Random|RandomIntegerinRange 0 (Utilities|Array|LastIndex (LocalVariables|GetInactiveCabinets)))))
  (if (Utilities|Array|IsValidIndex (LocalVariables|GetInactiveCabinets) _output_get)
    (Utilities|IsValid (Utilities|Array|Get(acopy) (LocalVariables|GetInactiveCabinets) (LocalVariables|GetRandomIndex))
      (:Is%20Valid
        (Class|BaseCabinet|ActivateCabinet (Utilities|Array|Get(acopy) (LocalVariables|GetInactiveCabinets) (LocalVariables|GetRandomIndex)))
        (return (Utilities|Array|Get(acopy) (LocalVariables|GetInactiveCabinets) (LocalVariables|GetRandomIndex))))
      (:Is%20Not%20Valid
        _)))
  (return 0))

(fn GetInactiveCabinets
  (for _array_element (Variables|Default|GetCabinets)
    (bind _returnvalue (Class|BaseCabinet|GetCurrentState _array_element))
    (if (Utilities|Name|Equal(Name) _returnvalue "Inactive")
      (Utilities|Array|AddUnique (LocalVariables|GetInactiveCabinets) _array_element)))
  (return (LocalVariables|GetInactiveCabinets)))

(fn UnlockDoors
  (for _array_element (Variables|Default|GetDoors)
    (Default|SetLocked _array_element false)))