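; MyBigGun is a big gun prop whose spin and sound follow the gun charge held by OnlyOneGameMode.
; Each charge update, including the initial one, plays a power-up sound and, once past a small threshold, fades in near and far spinning loops a single time.
; Tick eases intensity toward the charge, raising loop pitch and rotating two groups of gun parts in opposite directions at different speeds.
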(event Custom|UpdateIntensity
  (params (Charge :type Float%20%28single-precision%29))
  (bind _output_get (Variables|Default|SetTargetIntensity Charge))
  (Audio|SpawnSoundAttached "/Game/Audio/Audio_Assets/Ambience/Amb_Powerupbiggun_00_Cue.Amb_Powerupbiggun_00_Cue" (Variables|Default|GetGun_01) "None" "0, 0, 0" "0, 0, 0" "KeepRelativeOffset" false 1.0 1.0 0.0 0 0)
  (if (>= _output_get 0.08)
    (Utilities|FlowControl|DoOnce false
      (:Completed
        (Audio|Components|Audio|FadeIn (Variables|Default|Getbiggunspinning_far_loop_Cue) 2.0 1.0 0.0 :!class /Script/Engine.AudioComponent)
        (Audio|Components|Audio|FadeIn (Variables|Default|Getbiggunspinning_close_Loop) 2.0 1.0 0.0 :!class /Script/Engine.AudioComponent)))))

(event EventBeginPlay
  (bind _asonly_one_game_mode (Utilities|Casting|CastToOnlyOneGameMode (Game|GetGameMode)))
  (EventDispatchers|BindEventtoGunChargeChanged _asonly_one_game_mode (delegate Custom|UpdateIntensity))
  (CallFunction|UpdateIntensity (Variables|/Game/Blueprints/OnlyOneGameMode.OnlyOneGameMode_C|GetGunCharge _asonly_one_game_mode)))

(event EventTick
  (params (DeltaSeconds :type Float%20%28single-precision%29))
  (Utilities|FlowControl|Sequence
    (:then_0
      (bind _output_get (Variables|Default|SetCurrentIntensity (Math|Interpolation|FInterpTo (Variables|Default|GetCurrentIntensity) (Variables|Default|GetTargetIntensity) DeltaSeconds 5.0)))
      (Audio|Components|Audio|SetPitchMultiplier (Variables|Default|Getbiggunspinning_far_loop_Cue) (+ _output_get 1.0))
      (Audio|Components|Audio|SetPitchMultiplier (Variables|Default|Getbiggunspinning_close_Loop) (+ _output_get 1.0)))
    (:then_1
      (Transformation|AddLocalRotation (Variables|Default|GetGun_01) (Math|Rotator|MakeRotator 0.0 (* (* DeltaSeconds (Variables|Default|GetCurrentIntensity)) 1.2e+02) 0.0) false false)
      (Transformation|AddLocalRotation (Variables|Default|GetGun_04) (Math|Rotator|MakeRotator 0.0 (* (* DeltaSeconds (Variables|Default|GetCurrentIntensity)) -3.6e+02) 0.0) false false))))

(fn ConstructionScript)