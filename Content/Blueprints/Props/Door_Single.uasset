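; Sliding door prop that opens when the player character enters its trigger box and closes when they leave.
; One reversible timeline slides two panels along relative X, one travelling 2.1 times as far, while open and close sounds fade each other out.
; A lock blocks opening only, and SetLocked retries opening if the player is still in the box, so unlocking opens the door immediately.
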(event OnComponentBeginOverlap(Box)
  (params (OverlappedComponent :type Primitive%20Component%20Object%20Reference) (OtherActor :type Actor%20Object%20Reference) (OtherComp :type Primitive%20Component%20Object%20Reference) (OtherBodyIndex :type Integer) (bFromSweep :type Boolean) (SweepResult :type Hit%20Result%20Structure%20%28by%20ref%29))
  (Utilities|Casting|CastToPlayerCharacterBP OtherActor)
  (CallFunction|OpenDoor)
  (Variables|Default|SetWantsOpen true))

(event OnComponentEndOverlap(Box)
  (params (OverlappedComponent :type Primitive%20Component%20Object%20Reference) (OtherActor :type Actor%20Object%20Reference) (OtherComp :type Primitive%20Component%20Object%20Reference) (OtherBodyIndex :type Integer))
  (Utilities|Casting|CastToPlayerCharacterBP OtherActor)
  (CallFunction|CloseDoor)
  (Variables|Default|SetWantsOpen false))

(event Custom|OpenDoor
  (if (and (not (Variables|Default|GetIsLocked)) (not (Variables|Default|GetIsOpen)))
    (Variables|Default|SetIsOpen true)
    (Audio|Components|Audio|Play (Variables|Default|GetDoorOpen) 0.0)
    (Audio|Components|Audio|FadeOut (Variables|Default|GetDoorClose) 0.25 0.0 :!class /Script/Engine.AudioComponent)
    (bind _newtrack_0 (Timeline|DoorM Play)
      (:Update
        (Transformation|SetRelativeLocation (Variables|Default|GetDoorL_01) (Math|Vector|MakeVector (Math|Float|Lerp 0.0 -5e+01 _newtrack_0) 0.0 0.0) false false)
        (Transformation|SetRelativeLocation (Variables|Default|GetDoorM_01) (Math|Vector|MakeVector (* (Math|Float|Lerp 0.0 -5e+01 _newtrack_0) 2.1) 0.0 0.0) false false)))))

(event Custom|CloseDoor
  (if (Variables|Default|GetIsOpen)
    (Variables|Default|SetIsOpen false)
    (Audio|Components|Audio|Play (Variables|Default|GetDoorClose) 0.0)
    (Audio|Components|Audio|FadeOut (Variables|Default|GetDoorOpen) 0.25 0.0 :!class /Script/Engine.AudioComponent)
    (bind _newtrack_0 (Timeline|DoorM Reverse)
      (:Update
        (Transformation|SetRelativeLocation (Variables|Default|GetDoorL_01) (Math|Vector|MakeVector (Math|Float|Lerp 0.0 -5e+01 _newtrack_0) 0.0 0.0) false false)
        (Transformation|SetRelativeLocation (Variables|Default|GetDoorM_01) (Math|Vector|MakeVector (* (Math|Float|Lerp 0.0 -5e+01 _newtrack_0) 2.1) 0.0 0.0) false false)))))

(event EventBeginPlay)

(event Collision|EventActorBeginOverlap
  (params (OtherActor :type Actor%20Object%20Reference)))

(event EventTick
  (params (DeltaSeconds :type Float%20%28single-precision%29)))

(fn ConstructionScript)

(fn SetLocked
  (params (Locked :type Boolean))
  (Variables|Default|SetIsLocked Locked)
  (if (Variables|Default|GetWantsOpen)
    (CallFunction|OpenDoor)))