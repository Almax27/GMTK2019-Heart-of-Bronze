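; Double door prop built from two Door_Single child actors, left and right, with locked-state text on the front and back.
; SetLocked forwards the locked state to both child doors and shows or hides both text components to match.
; The BeginLocked setting is applied in the construction script and again at BeginPlay.
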(event EventBeginPlay
  (CallFunction|SetLocked (Variables|Default|GetBeginLocked)))

(fn ConstructionScript
  (CallFunction|SetLocked (Variables|Default|GetBeginLocked)))

(fn SetLocked
  (params (Locked :type Boolean))
  (Utilities|FlowControl|Sequence
    (:then_0
      (bind _asdoor_single (Utilities|Casting|CastToDoor_Single (Variables|/Script/Engine.ChildActorComponent|GetChildActor (Variables|Default|GetRightDoor))))
      (Default|SetLocked _asdoor_single Locked)
      (bind _asdoor_single_2 (Utilities|Casting|CastToDoor_Single (Variables|/Script/Engine.ChildActorComponent|GetChildActor (Variables|Default|GetLeftDoor))))
      (Default|SetLocked _asdoor_single_2 Locked))
    (:then_1
      (Rendering|SetVisibility (Variables|Default|GetLockedTextFront) Locked false))))