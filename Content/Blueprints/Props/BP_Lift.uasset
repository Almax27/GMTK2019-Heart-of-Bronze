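; Elevator prop that carries the player between an upper and lower stop, starting gated until an Unlock event clears it.
; Player overlap on the trigger enables blocking collision and chains gate and lift timelines, lerping relative Z and playing forward or reverse based on LiftIsUp.
; On arrival it flips that state, crossfades machinery audio, fades out the music, removes blocking and reverses the gate timeline.
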(event OnComponentBeginOverlap(Trigger)
  (params (OverlappedComponent :type Primitive%20Component%20Object%20Reference) (OtherActor :type Actor%20Object%20Reference) (OtherComp :type Primitive%20Component%20Object%20Reference) (OtherBodyIndex :type Integer) (bFromSweep :type Boolean) (SweepResult :type Hit%20Result%20Structure%20%28by%20ref%29))
  (Utilities|Casting|CastToPlayerCharacterBP OtherActor)
  (if (not (Variables|Default|GetIsLiftTraveling))
    (Variables|Default|SetIsLiftTraveling true)
    (Collision|SetCollisionEnabled (Variables|Default|GetBlocking) "QueryAndPhysics")
    (Audio|Components|Audio|FadeIn (Variables|Default|Getelevator%20tune) 1.0 1.0 0.0 :!class /Script/Engine.AudioComponent)
    (Audio|Components|Audio|Play (Variables|Default|GetAmb_Hiss_Oneshot_01) 0.0)
    (Audio|Components|Audio|Play (Variables|Default|Getelevator%20start) 0.0)
    (bind (_direction _liftheight) (Timeline|LiftGateAnimation Play)
      (:Update
        (Transformation|SetRelativeLocation (Variables|Default|GetLiftGate) (Math|Vector|MakeVector 0.0 0.0 (Math|Float|Lerp -1.5e+02 0.0 _liftheight)) false false))
      (:Finished
        (switch Utilities|FlowControl|Switch|SwitchonETimelineDirection _direction
          (:Forward
            (if (Variables|Default|GetLiftIsUp)
              (bind _liftheight_2 (Timeline|LiftAnimationTimeline Play)
                (:Update
                  (Transformation|SetRelativeLocation (Variables|Default|GetLift) (Math|Vector|MakeVector 0.0 0.0 (Math|Float|Lerp 0.0 -7.1e+03 _liftheight_2)) false false))
                (:Finished
                  (Variables|Default|SetLiftIsUp (not (Variables|Default|GetLiftIsUp)))
                  (Audio|Components|Audio|FadeOut (Variables|Default|Getelevator%20start) 0.5 0.0 :!class /Script/Engine.AudioComponent)
                  (Audio|Components|Audio|FadeIn (Variables|Default|Getelevator_Stop_Machinery_00_Cue) 0.5 1.0 0.0 :!class /Script/Engine.AudioComponent)
                  (Audio|Components|Audio|Play (Variables|Default|Getelevator_thump_Cue) 0.0)
                  (CallFunction|LiftFInishedTraveling)))
              (else
                (Timeline|LiftAnimationTimeline Reverse)))))))))

(event Custom|LiftFInishedTraveling
  (Variables|Default|SetIsLiftTraveling false)
  (Audio|Components|Audio|FadeOut (Variables|Default|Getelevator%20tune) 3.0 0.0 :!class /Script/Engine.AudioComponent)
  (Collision|SetCollisionEnabled (Variables|Default|GetBlocking) "NoCollision")
  (bind (_direction _liftheight) (Timeline|LiftGateAnimation Reverse)
    (:Update
      (Transformation|SetRelativeLocation (Variables|Default|GetLiftGate) (Math|Vector|MakeVector 0.0 0.0 (Math|Float|Lerp -1.5e+02 0.0 _liftheight)) false false))
    (:Finished
      (switch Utilities|FlowControl|Switch|SwitchonETimelineDirection _direction
        (:Forward
          (if (Variables|Default|GetLiftIsUp)
            (bind _liftheight_2 (Timeline|LiftAnimationTimeline Play)
              (:Update
                (Transformation|SetRelativeLocation (Variables|Default|GetLift) (Math|Vector|MakeVector 0.0 0.0 (Math|Float|Lerp 0.0 -7.1e+03 _liftheight_2)) false false))
              (:Finished
                (Variables|Default|SetLiftIsUp (not (Variables|Default|GetLiftIsUp)))
                (Audio|Components|Audio|FadeOut (Variables|Default|Getelevator%20start) 0.5 0.0 :!class /Script/Engine.AudioComponent)
                (Audio|Components|Audio|FadeIn (Variables|Default|Getelevator_Stop_Machinery_00_Cue) 0.5 1.0 0.0 :!class /Script/Engine.AudioComponent)
                (Audio|Components|Audio|Play (Variables|Default|Getelevator_thump_Cue) 0.0)
                (CallFunction|LiftFInishedTraveling)))
            (else
              (Timeline|LiftAnimationTimeline Reverse))))))))

(event Custom|Unlock
  (Collision|SetCollisionEnabled (Variables|Default|GetBlocking) "NoCollision")
  (bind _liftheight (Timeline|Timeline_0 Reverse)
    (:Update
      (Transformation|SetRelativeLocation (Variables|Default|GetLiftGate) (Math|Vector|MakeVector 0.0 0.0 (Math|Float|Lerp -1.5e+02 0.0 _liftheight)) false false))))

(event EventBeginPlay
  (Collision|SetCollisionEnabled (Variables|Default|GetBlocking) "QueryAndPhysics")
  (bind _liftheight (Timeline|Timeline_0 SetNewTime)
    (:Update
      (Transformation|SetRelativeLocation (Variables|Default|GetLiftGate) (Math|Vector|MakeVector 0.0 0.0 (Math|Float|Lerp -1.5e+02 0.0 _liftheight)) false false))))

(fn ConstructionScript)

(fn SetLocked)