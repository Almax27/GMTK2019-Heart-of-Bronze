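; Alarm light prop that switches between a critical and a non-critical look through the UpdateCriticalState event.
; When critical, it shows two spotlights, sets the cube's BaseColor material parameter to the critical color and plays a timeline that drives the cube's yaw.
; When not critical, it hides the spotlights, applies the non-critical color and stops the timeline.
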(event EventUpdateCriticalState
  (params (IsCritical :type Boolean))
  (bind _cube (Variables|Default|GetCube))
  (bind _relativerotation (Variables|/Script/Engine.SceneComponent|GetRelativeRotation _cube))
  (bind (_roll _pitch) (Math|Rotator|BreakRotator _relativerotation))
  (Utilities|FlowControl|Sequence
    (:then_0
      (Rendering|SetVisibility (Variables|Default|GetSpotLight2) IsCritical false)
      (Rendering|Material|SetVectorParameterValueonMaterials (Variables|Default|GetCube) "BaseColor" (Math|Conversions|ToVector(LinearColor) (Math|Color|SelectColor (Variables|Default|GetCriticalColor) (Variables|Default|GetNonCriticalColor) IsCritical))))
    (:then_1
      (if IsCritical
        (bind _yaw (Timeline|Timeline_0 Play)
          (:Update
            (Transformation|SetRelativeRotation _cube (Math|Rotator|MakeRotator _roll _pitch _yaw) false false)))
        (else
          (Timeline|Timeline_0 Stop))))))

(fn ConstructionScript)