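; Game event for the shield-failure game over, which plays the loss voice-over and returns the game to the title screen.
; On begin it plays the shield failure line, then follows it with a randomly chosen generic loss line.
; A PendingEnd flag lets the single dialogue-finished callback tell the two lines apart and end the event after the second.
; On end it calls the parent, then asks OnlyOneGameMode to return to title.
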(event EventOnBegin
  (Variables|Default|SetPendingEnd false)
  (CallFunction|PlayDialogue "/Game/Audio/Audio_Assets/Dialogue/VO_GameOver_ShieldFailure.VO_GameOver_ShieldFailure"))

(event EventOnDialogueFinished
  (if (Variables|Default|GetPendingEnd)
    (Class|GameEvent|End)
    (else
      (Variables|Default|SetPendingEnd true)
      (CallFunction|PlayRandomDialogue (Utilities|Array|MakeArray "/Game/Audio/Audio_Assets/Dialogue/VO_GameOver_Loss01.VO_GameOver_Loss01" "/Game/Audio/Audio_Assets/Dialogue/VO_GameOver_Loss02.VO_GameOver_Loss02" "/Game/Audio/Audio_Assets/Dialogue/VO_GameOver_Loss03.VO_GameOver_Loss03" "/Game/Audio/Audio_Assets/Dialogue/VO_GameOver_Loss04.VO_GameOver_Loss04")))))

(event EventOnEnd
  (|CallParentFunction)
  (bind _asonly_one_game_mode (Utilities|Casting|CastToOnlyOneGameMode (Game|GetGameMode)))
  (Default|ReturntoTitleScreen _asonly_one_game_mode))