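; NavigationEvent is a game event that gives the player a cabinet task in the navigation room.
; On begin it plays a missile event voice line, then activates the Cabinet from the NavigationRoomManager, if valid, and binds to its result delegate.
; When the cabinet reports a result, it unbinds and ends the event without checking the outcome.
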(event Custom|OnResult
  (params (result :type Cabinet%20Result%20Structure))
  (EventDispatchers|UnbindEventfromOnCabinetResult (.Cabinet (Utilities|Struct|BreakCabinetResult result)) (delegate Custom|OnResult))
  (Class|GameEvent|End))

(event EventOnBegin
  (CallFunction|PlayDialogue "/Game/Audio/Audio_Assets/Dialogue/VO_MissileEvent01.VO_MissileEvent01")
  (bind _manager (CallFunction|GetNavigationRoomManager self))
  (Utilities|IsValid _manager
    (:Is%20Valid
      (Class|BaseCabinet|ActivateCabinet (Variables|/Game/Blueprints/Gameplay/NavigationRoomManager.NavigationRoomManager_C|GetCabinet _manager))
      (EventDispatchers|BindEventtoOnCabinetResult (Variables|/Game/Blueprints/Gameplay/NavigationRoomManager.NavigationRoomManager_C|GetCabinet _manager) (delegate Custom|OnResult)))))