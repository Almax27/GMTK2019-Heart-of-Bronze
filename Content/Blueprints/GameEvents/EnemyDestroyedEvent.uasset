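; Game event that plays the victory sequence after the enemy is destroyed, then returns the game to the title screen.
; On begin it plays the enemy-destroyed voice line, and when that finishes it follows with a randomly chosen win line.
; A PendingEnd flag lets the single dialogue-finished callback tell the two lines apart and end the event after the second.
; On end, it asks OnlyOneGameMode to return to the title screen.
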(event EventOnBegin
  (Variables|Default|SetPendingEnd false)
  (CallFunction|PlayDialogue "/Game/Audio/Audio_Assets/Dialogue/VO_GameOver_EnemyDestroyed.VO_GameOver_EnemyDestroyed"))

(event EventOnDialogueFinished
  (if (Variables|Default|GetPendingEnd)
    (Class|GameEvent|End)
    (else
      (Variables|Default|SetPendingEnd true)
      (CallFunction|PlayRandomDialogue (Utilities|Array|MakeArray "/Game/Audio/Audio_Assets/Dialogue/VO_GameOver_Win01.VO_GameOver_Win01" "/Game/Audio/Audio_Assets/Dialogue/VO_GameOver_Win02.VO_GameOver_Win02" "/Game/Audio/Audio_Assets/Dialogue/VO_GameOver_Win03.VO_GameOver_Win03" "/Game/Audio/Audio_Assets/Dialogue/VO_GameOver_Win04.VO_GameOver_Win04")))))

(event EventOnEnd
  (|CallParentFunction)
  (bind _asonly_one_game_mode (Utilities|Casting|CastToOnlyOneGameMode (Game|GetGameMode)))
  (Default|ReturntoTitleScreen _asonly_one_game_mode))