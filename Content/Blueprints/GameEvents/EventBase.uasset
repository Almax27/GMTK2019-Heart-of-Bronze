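; EventBase is a base Blueprint for game events that provides begin and end hooks plus 2D dialogue playback.
; PlayDialogue stops any active line, fires an interruption hook, then spawns the new sound and binds to its audio-finished delegate.
; OnDialogueFinished clears the stored audio component and also runs when spawning fails, while OnEnd unbinds and stops playback.
; PlayRandomDialogue picks a random sound from an array for PlayDialogue.
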(event Custom|OnDialogueFinished
  (Variables|Transient|SetAudioComponent 0))

(event Custom|PlayDialogue
  (params (DialogueSound :type Sound%20Wave%20Object%20Reference))
  (Utilities|FlowControl|Sequence
    (:then_0
      (Utilities|IsValid (Variables|Transient|GetAudioComponent)
        (:Is%20Valid
          (EventDispatchers|UnbindEventfromOnAudioFinished (Variables|Transient|GetAudioComponent) (EventDispatchers|CreateEvent :!event Custom|OnDialogueFinished))
          (Audio|Components|Audio|Stop (Variables|Transient|GetAudioComponent))
          (CallFunction|OnDialogueInterupted))))
    (:then_1
      (bind _returnvalue (Audio|SpawnSound2D DialogueSound 1.0 1.0 0.0 0))
      (bind _output_get (Variables|Transient|SetAudioComponent _returnvalue))
      (Utilities|IsValid _output_get
        (:Is%20Valid
          (EventDispatchers|BindEventtoOnAudioFinished (Variables|Transient|GetAudioComponent) (EventDispatchers|CreateEvent :!event Custom|OnDialogueFinished)))
        (:Is%20Not%20Valid
          (CallFunction|OnDialogueFinished))))))

(event Custom|OnDialogueInterupted)

(event EventOnBegin)

(event EventOnEnd
  (bind _audiocomponent (Variables|Transient|GetAudioComponent))
  (Utilities|IsValid _audiocomponent
    (:Is%20Valid
      (EventDispatchers|UnbindEventfromOnAudioFinished _audiocomponent (EventDispatchers|CreateEvent :!event Custom|OnDialogueFinished))
      (Audio|Components|Audio|Stop _audiocomponent))))

(fn PlayRandomDialogue
  (params (Sounds :type Array%20of%20Sound%20Wave%20Object%20References))
  (bind _returnvalue (Utilities|Array|Length Sounds))
  (if (> _returnvalue 0)
    (CallFunction|PlayDialogue (Utilities|Array|Get(acopy) Sounds (Math|Random|RandomIntegerinRange 0 (- _returnvalue 1))))))