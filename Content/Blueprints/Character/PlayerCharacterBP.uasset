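; Player character Blueprint handling move, look, jump and sprint input, movement audio, camera head bob and the possession-bound HUD.
; Tick updates walk speed, allowing held or toggled sprint only when moving fast with forward input; state changes drive breath, clothing and footstep audio.
; Velocity scales head-bob camera shakes and the play rate of a timeline that triggers grounded footsteps.
; SlowInputForDuration temporarily scales look and move input through a retriggerable delay.
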(event Custom|OnSprintChanged
  (bind _outofbreathsound (Variables|Default|GetOutOfBreathSound))
  (Utilities|FlowControl|Sequence
    (:then_0
      (if (Variables|Transient|GetIsSprinting)
        (Audio|Components|Audio|FadeIn _outofbreathsound 1e+01 1.0 0.0 :!class /Script/Engine.AudioComponent)
        (Audio|SpawnSoundAttached "/Game/Audio/Audio_Assets/Foley/foot/Fol_Walk_Clothes_00_Cue.Fol_Walk_Clothes_00_Cue" (Variables|Collision|GetCapsuleComponent) "None" "0, 0, 0" "0, 0, 0" "KeepRelativeOffset" false 0.3 1.0 0.0 0 0)
        (Audio|Parameter|SetFloatParameter (Variables|Default|GetFootStepSound) "None" 1.0 :!class /Script/Engine.AudioComponent)
        (else
          (Audio|Components|Audio|FadeOut _outofbreathsound 4.0 0.0 :!class /Script/Engine.AudioComponent)
          (Audio|Parameter|SetFloatParameter (Variables|Default|GetFootStepSound) "None" 0.0 :!class /Script/Engine.AudioComponent))))))

(event Custom|SlowInputForDuration
  (params (LookScalar :type Float%20%28single-precision%29) (MoveScalar :type Float%20%28single-precision%29) (Duration :type Float%20%28single-precision%29))
  ;[1 1 1] Input
  (Variables|Transient|SetLookInputScalar LookScalar)
  (Variables|Transient|SetMoveInputScalar MoveScalar)
  (Utilities|FlowControl|RetriggerableDelay Duration)
  (Variables|Transient|SetLookInputScalar 1.0)
  (Variables|Transient|SetMoveInputScalar 1.0))

(event EventTick
  (params (DeltaSeconds :type Float%20%28single-precision%29))
  (CallFunction|UpdateWalkSpeed DeltaSeconds)
  (CallFunction|UpdateHeadBob DeltaSeconds)
  (Components|Timeline|SetPlayRate (Variables|Default|GetFootStepTimeline) (/ (Math|Vector|VectorLengthXY (Transformation|GetVelocity)) 2e+02)))

(event EventPossessed
  (params (NewController :type Controller%20Object%20Reference))
  (bind _asplayer_controller (Utilities|Casting|CastToPlayerController NewController))
  (CallFunction|AddHud _asplayer_controller))

(event EventUnpossessed
  (params (OldController :type Controller%20Object%20Reference))
  (CallFunction|RemoveHud))

(event EventOnLanded
  (params (Hit :type Hit%20Result%20Structure%20%28by%20ref%29))
  (Audio|SpawnSoundAttached "/Game/Audio/Audio_Assets/Foley/foot/Fol_land_00_Cue.Fol_land_00_Cue" (Variables|Collision|GetCapsuleComponent) "None" "0, 0, 0" "0, 0, 0" "KeepRelativeOffset" false 1.0 1.0 0.0 0 0))

(event EventOnJumped
  (Audio|SpawnSoundAttached "/Game/Audio/Audio_Assets/Foley/foot/Fol_Jump_00_Cue.Fol_Jump_00_Cue" (Variables|Collision|GetCapsuleComponent) "None" "0, 0, 0" "0, 0, 0" "KeepRelativeOffset" false 0.5 1.0 0.0 0 0))

(event EventBeginPlay
  ;[1 1 1] Footstep timeline
  (Timeline|FootStepTimeline PlayFromStart
    (:FootStepEvent
      (if (AI|Components|NavMovement|IsMovingonGround (Variables|Character|GetCharacterMovement))
        (Audio|Components|Audio|Play (Variables|Default|GetFootStepSound) 0.0)))))

(event Input|ActionEvents|InputActionJump
  (params (Key :type Key%20Structure))
  ;[1 1 1] Input
  (:Pressed
    (Character|Jump))
  (:Released
    (Character|StopJumping)))

(event Input|ActionEvents|InputActionSprintToggle
  (params (Key :type Key%20Structure))
  ;[1 1 1] Input
  (:Pressed
    (Variables|Transient|SetIsSprintToggled true)))

(event Input|ActionEvents|InputActionSprint
  (params (Key :type Key%20Structure))
  ;[1 1 1] Input
  (:Pressed
    (Variables|Transient|SetIsSprintPressed true))
  (:Released
    (Variables|Transient|SetIsSprintPressed false)))

(event Input|AxisEvents|InputAxisMoveForward
  (params (AxisValue :type Float%20%28single-precision%29))
  ;[1 1 1] Input
  (Pawn|Input|AddMovementInput (Transformation|GetActorForwardVector) (CallFunction|ScaleInput AxisValue true) false))

(event Input|AxisEvents|InputAxisMoveRight
  (params (AxisValue :type Float%20%28single-precision%29))
  ;[1 1 1] Input
  (Pawn|Input|AddMovementInput (Transformation|GetActorRightVector) (CallFunction|ScaleInput AxisValue true) false))

(event Input|AxisEvents|InputAxisLookUp
  (params (AxisValue :type Float%20%28single-precision%29))
  ;[1 1 1] Input
  (Pawn|Input|AddControllerPitchInput (CallFunction|ScaleInput AxisValue false)))

(event Input|AxisEvents|InputAxisLookRight
  (params (AxisValue :type Float%20%28single-precision%29))
  ;[1 1 1] Input
  (Pawn|Input|AddControllerYawInput (CallFunction|ScaleInput AxisValue false)))

(fn ConstructionScript)

(fn UpdateWalkSpeed
  (params (DeltaTime :type Float%20%28single-precision%29))
  (LocalVariables|SetWasSprinting (Variables|Transient|GetIsSprinting))
  (LocalVariables|SetCanSprint (and (> (Math|Vector|VectorLengthXY (Variables|/Script/Engine.MovementComponent|GetVelocity (Variables|Character|GetCharacterMovement))) 3e+02) (> (Class|KismetMathLibrary|VectorCosineAngle2D (Transformation|GetActorForwardVector) (Pawn|Components|PawnMovement|GetLastInputVector (Variables|Character|GetCharacterMovement))) 0.5)))
  (Utilities|FlowControl|Sequence
    (:then_0
      (Utilities|FlowControl|Sequence
        (:then_0
          (if (Variables|Transient|GetIsSprintToggled)
            (Variables|Transient|SetIsSprintToggled (LocalVariables|GetCanSprint))))
        (:then_1
          (if (Variables|Transient|GetIsSprintPressed)
            _))))
    (:then_1
      (Variables|Transient|SetIsSprinting (and (LocalVariables|GetCanSprint) (or (Variables|Transient|GetIsSprintToggled) (Variables|Transient|GetIsSprintPressed)))))
    (:then_2
      (Variables|/Script/Engine.CharacterMovementComponent|SetMaxWalkSpeed (Variables|Character|GetCharacterMovement) (select (Variables|Transient|GetIsSprinting) (Variables|Default|GetMaxSprintSpeed) (Variables|Default|GetMaxWalkSpeed))))
    (:then_3
      (if (Math|Boolean|NotEqual(Boolean) (Variables|Transient|GetIsSprinting) (LocalVariables|GetWasSprinting))
        (CallFunction|OnSprintChanged)))))

(fn UpdateHeadBob
  (params (DeltaTime :type Float%20%28single-precision%29))
  (bind _charactermovement (Variables|Character|GetCharacterMovement))
  (bind _returnvalue (Class|MovementComponent|GetMaxSpeed _charactermovement))
  (bind _velocity (Variables|/Script/Engine.MovementComponent|GetVelocity _charactermovement))
  (bind _returnvalue_2 (Math|Vector|VectorLengthXY _velocity))
  (bind _returnvalue_3 (/ _returnvalue_2 _returnvalue))
  (bind _asplayer_controller (Utilities|Casting|CastToPlayerController (Pawn|GetController)))
  (if (Variables|Transient|GetIsSprinting)
    (Class|PlayerController|ClientPlayCameraShake _asplayer_controller "/Game/Blueprints/Character/CamShakeSprint.CamShakeSprint_C" (* _returnvalue_3 1.5) "CameraLocal" "0, 0, 0")
    (Game|Feedback|ClientStopCameraShake _asplayer_controller "/Game/Blueprints/Character/CamShakeRun.CamShakeRun_C" false)
    (else
      (Class|PlayerController|ClientPlayCameraShake _asplayer_controller "/Game/Blueprints/Character/CamShakeRun.CamShakeRun_C" _returnvalue_3 "CameraLocal" "0, 0, 0")
      (Game|Feedback|ClientStopCameraShake _asplayer_controller "/Game/Blueprints/Character/CamShakeSprint.CamShakeSprint_C" false))))

(fn AddHud
  (params (PlayerController :type Player%20Controller%20Object%20Reference))
  (bind _returnvalue (UserInterface|CreateWidget (Variables|Default|GetPlayerHUDClass) PlayerController))
  (Utilities|IsValid _returnvalue
    (:Is%20Valid
      (bind _output_get (Variables|Default|SetPlayerHUD _returnvalue))
      (bind _asplayer_hud (Utilities|Casting|CastToPlayerHUD _output_get))
      (Default|OnShow _asplayer_hud)
      (UserInterface|Viewport|AddtoViewport _output_get 0))))

(fn RemoveHud
  (Widget|RemovefromParent (Variables|Default|GetPlayerHUD))
  (Variables|Default|SetPlayerHUD 0))

(fn ScaleInput
  (params (Raw :type Float%20%28single-precision%29) (IsMove :type Boolean))
  (return (* Raw (select IsMove (Variables|Transient|GetMoveInputScalar) (Variables|Transient|GetLookInputScalar)))))