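; Player controller that drives look-at highlighting and interaction, plus developer debug hotkeys.
; Each tick a camera trace tracks the component in view, sending highlight changes through InteractableInterface on its owner or itself and to the player HUD.
; The Interact input repeats the trace and calls OnInteract on the hit actor and component.
; Hotkeys, gated by DebugExec to non-distribution builds, spawn explosions, change levels and poke game mode events, ship health and gun charge.
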(event EventTick
  (params (DeltaSeconds :type Float%20%28single-precision%29))
  (bind _playercameramanager (Variables|Default|GetPlayerCameraManager))
  (bind _returnvalue (Transformation|GetActorLocation _playercameramanager))
  (bind _outhit (Collision|LineTraceByChannel _returnvalue (+ _returnvalue (* (Transformation|GetActorForwardVector _playercameramanager) (Variables|Default|GetInteractDistance))) "TraceTypeQuery1" true 0 "None"))
  (if (!= (.HitComponent (Collision|BreakHitResult _outhit)) (Variables|Transient|GetHighlightedComponent))
    (Utilities|FlowControl|Sequence
      (:then_0
        (Utilities|IsValid (Variables|Transient|GetHighlightedComponent)
          (:Is%20Valid
            (Utilities|FlowControl|Sequence
              (:then_0
                (bind _asinteractable_interface (Utilities|Casting|CastToInteractableInterface (Components|GetOwner (Variables|Transient|GetHighlightedComponent))))
                (Class|InteractableInterface|OnEndHighlight _asinteractable_interface (Variables|Transient|GetHighlightedComponent)))
              (:then_1
                (bind _asinteractable_interface_2 (Utilities|Casting|CastToInteractableInterface (Variables|Transient|GetHighlightedComponent)))
                (Class|InteractableInterface|OnEndHighlight _asinteractable_interface_2 (Variables|Transient|GetHighlightedComponent))))
            (bind _asplayer_character_bp (Utilities|Casting|CastToPlayerCharacterBP (Game|GetPlayerCharacter 0)))
            (bind _asplayer_hud (Utilities|Casting|CastToPlayerHUD (Variables|/Game/Blueprints/Character/PlayerCharacterBP.PlayerCharacterBP_C|GetPlayerHUD _asplayer_character_bp)))
            (Default|OnEndHighlight _asplayer_hud))))
      (:then_1
        (Variables|Transient|SetHighlightedComponent (.HitComponent (Collision|BreakHitResult _outhit))))
      (:then_2
        (Utilities|IsValid (Variables|Transient|GetHighlightedComponent)
          (:Is%20Valid
            (Utilities|FlowControl|Sequence
              (:then_0
                (bind _asinteractable_interface_3 (Utilities|Casting|CastToInteractableInterface (Components|GetOwner (Variables|Transient|GetHighlightedComponent))))
                (Class|InteractableInterface|OnBeginHighlight _asinteractable_interface_3 (Variables|Transient|GetHighlightedComponent)))
              (:then_1
                (bind _asinteractable_interface_4 (Utilities|Casting|CastToInteractableInterface (Variables|Transient|GetHighlightedComponent)))
                (Class|InteractableInterface|OnBeginHighlight _asinteractable_interface_4 (Variables|Transient|GetHighlightedComponent))))
            (bind _asplayer_character_bp_2 (Utilities|Casting|CastToPlayerCharacterBP (Game|GetPlayerCharacter 0)))
            (bind _asplayer_hud_2 (Utilities|Casting|CastToPlayerHUD (Variables|/Game/Blueprints/Character/PlayerCharacterBP.PlayerCharacterBP_C|GetPlayerHUD _asplayer_character_bp_2)))
            (Default|OnBeginHighlight _asplayer_hud_2)))))))

(event Input|ActionEvents|InputActionInteract
  (params (Key :type Key%20Structure))
  (bind _playercameramanager (Variables|Default|GetPlayerCameraManager))
  (bind _returnvalue (Transformation|GetActorLocation _playercameramanager))
  (:Pressed
    (bind (_outhit _returnvalue_2) (Collision|LineTraceByChannel _returnvalue (+ _returnvalue (* (Transformation|GetActorForwardVector _playercameramanager) (Variables|Default|GetInteractDistance))) "TraceTypeQuery1" true 0 "None"))
    (if _returnvalue_2
      (Utilities|FlowControl|Sequence
        (:then_0
          (bind _asinteractable_interface (Utilities|Casting|CastToInteractableInterface (.HitActor (Collision|BreakHitResult _outhit))))
          (Class|InteractableInterface|OnInteract _asinteractable_interface _outhit))
        (:then_1
          (bind _asinteractable_interface_2 (Utilities|Casting|CastToInteractableInterface (.HitComponent (Collision|BreakHitResult _outhit))))
          (Class|InteractableInterface|OnInteract _asinteractable_interface_2 _outhit))))))

(event Input|KeyboardEvents|R
  (params (Key :type Key%20Structure))
  (:Pressed
    (Utilities|DebugExec
      (:Out
        (bind _returnvalue (Game|GetCurrentLevelName true))
        (Game|OpenLevel(byName) (Utilities|String|StringToName _returnvalue))))))

(event Input|KeyboardEvents|NumPadTwo
  (params (Key :type Key%20Structure))
  (:Pressed
    (Utilities|DebugExec
      (:Out
        (Game|SpawnActorfromClass "/Game/Blueprints/Gameplay/MissileExplosion.MissileExplosion_C" (Math|Transform|MakeTransform (+ (Transformation|GetActorLocation (Pawn|GetControlledPawn)) (* (Math|Random|RandomUnitVector) 1e+03))) "AlwaysSpawn" 0 0)))))

(event Input|KeyboardEvents|NumPadOne
  (params (Key :type Key%20Structure))
  (:Pressed
    (Utilities|DebugExec
      (:Out
        (Game|SpawnActorfromClass "/Game/Blueprints/Gameplay/MissileExplosion.MissileExplosion_C" (Math|Transform|MakeTransform (+ (Transformation|GetActorLocation (Pawn|GetControlledPawn)) (* (Math|Random|RandomUnitVector) 1e+03))) "AlwaysSpawn" 0 0)))))

(event Input|KeyboardEvents|#
  (params (Key :type Key%20Structure))
  (:Pressed
    (Utilities|DebugExec
      (:Out
        (bind _asonly_one_game_mode (Utilities|Casting|CastToOnlyOneGameMode (Game|GetGameMode)))
        (Default|TakeShipDamage _asonly_one_game_mode 0.1)))))

(event Input|KeyboardEvents|1
  (params (Key :type Key%20Structure))
  (:Pressed
    (Utilities|DebugExec
      (:Out
        (bind _asonly_one_game_mode (Utilities|Casting|CastToOnlyOneGameMode (Game|GetGameMode)))
        (Class|GMTKJam2019GameModeBase|SubmitGameEventbyName _asonly_one_game_mode "Test1")))))

(event Input|KeyboardEvents|2
  (params (Key :type Key%20Structure))
  (:Pressed
    (Utilities|DebugExec
      (:Out
        (bind _asonly_one_game_mode (Utilities|Casting|CastToOnlyOneGameMode (Game|GetGameMode)))
        (Class|GMTKJam2019GameModeBase|SubmitGameEventbyName _asonly_one_game_mode "Test2")))))

(event Input|KeyboardEvents|3
  (params (Key :type Key%20Structure))
  (:Pressed
    (Utilities|DebugExec
      (:Out
        (bind _asonly_one_game_mode (Utilities|Casting|CastToOnlyOneGameMode (Game|GetGameMode)))
        (Class|GMTKJam2019GameModeBase|SubmitGameEventbyName _asonly_one_game_mode "Test3")))))

(event Input|KeyboardEvents|H
  (params (Key :type Key%20Structure))
  (:Pressed
    (Utilities|DebugExec
      (:Out
        (bind _asonly_one_game_mode (Utilities|Casting|CastToOnlyOneGameMode (Game|GetGameMode)))
        (Default|ResetShipHealth _asonly_one_game_mode)))))

(event Input|KeyboardEvents|I
  (params (Key :type Key%20Structure))
  (:Pressed
    (Utilities|DebugExec
      (:Out
        (bind _asonly_one_game_mode (Utilities|Casting|CastToOnlyOneGameMode (Game|GetGameMode)))
        (Default|AddGunCharge _asonly_one_game_mode 0.2)))))

(event Input|KeyboardEvents|T
  (params (Key :type Key%20Structure))
  (:Pressed
    (Utilities|DebugExec
      (:Out
        (bind _asonly_one_game_mode (Utilities|Casting|CastToOnlyOneGameMode (Game|GetGameMode)))
        (Default|ReturntoTitleScreen _asonly_one_game_mode)))))

(fn ConstructionScript)