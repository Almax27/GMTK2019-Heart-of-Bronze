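; A cabinet Blueprint built around a single push button, which reports success when pressed while the cabinet is active.
; On BeginPlay it binds to the press dispatcher of its ButtonBP child actor; each press sets a flag and runs the parent-derived result check.
; Success broadcasts a result, switches to Inactive and plays a sound; presses in other states play a non-interactive sound.
; State changes clear the pressed flag.
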(event Custom|OnReceiveButtonPress
  ;[1 1 1] Handle receipt of button press by calling OnButtonPressed
  (Variables|Transient|SetButtonPressed true)
  (Utilities|FlowControl|Sequence
    (:then_0
      (bind _returnvalue (Class|BaseCabinet|GetCurrentState))
      (if (not (Utilities|Name|Equal(Name) _returnvalue "Active"))
        (Audio|PlaySoundatLocation "/Game/Audio/Last_bits/Noninteractivebutton.Noninteractivebutton" "0, 0, 0" "0, 0, 0" 0.2 1.0 0.0 0 0 0)))
    (:then_1
      (Class|BaseCabinet|CheckforResult))))

(event EventBeginPlay
  (|CallParentFunction)
  (bind _asbutton_bp (Utilities|Casting|CastToButtonBP (Variables|/Script/Engine.ChildActorComponent|GetChildActor (Variables|Default|GetButton))))
  (EventDispatchers|BindEventtoOnButtonPressed _asbutton_bp (EventDispatchers|CreateEvent :!event Custom|OnReceiveButtonPress)))

(event Collision|EventActorBeginOverlap
  (params (OtherActor :type Actor%20Object%20Reference)))

(event EventTick
  (params (DeltaSeconds :type Float%20%28single-precision%29)))

(event EventCheckforResult
  (|CallParentFunction)
  (bind _returnvalue (Class|BaseCabinet|GetCurrentState))
  (if (and (Variables|Transient|GetButtonPressed) (Utilities|Name|Equal(Name) _returnvalue "Active"))
    (Class|BaseCabinet|BroadcastResult (Utilities|Struct|MakeCabinetResult "Success"))
    (Class|BaseCabinet|ChangeState "Inactive")
    (Audio|PlaySoundatLocation "/Game/Audio/Audio_Assets/minigames/UI_Minigames_Correct_Square_00.UI_Minigames_Correct_Square_00" (Transformation|GetWorldLocation (Variables|Default|GetButton_Holder)) "0, 0, 0" 1.0 1.0 0.0 0 0 0)))

(event EventActivateCabinet
  (|CallParentFunction))

(event EventOnStateChanged
  (params (cabinet :type Base%20Cabinet%20Object%20Reference))
  (|CallParentFunction cabinet)
  (Class|BaseCabinet|GetCurrentState)
  (Variables|Transient|SetButtonPressed false))

(fn ConstructionScript)