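; NavigationCabinetBP is a ship cabinet minigame where left and right buttons switch lanes to dodge incoming missile salvos.
; While Active, it ticks its NavigationComponent and shows the monitor widget, growing the salvo size with each activation up to a cap.
; Impacts in the current lane damage the ship through OnlyOneGameMode and spawn an explosion around the player.
; The last impact deactivates the cabinet and reports Success, even after hits.
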(event Custom|OnRightButtonPressed
  (Class|NavigationComponent|ChangeLane (Variables|Default|GetNavigationComponent) true))

(event Custom|OnLeftButtonPressed
  (Class|NavigationComponent|ChangeLane (Variables|Default|GetNavigationComponent) false))

(event Custom|OnMissileImpactEvent
  (params (missile :type Missile%20Structure))
  (bind _returnvalue (Class|NavigationComponent|GetCurrentLane (Variables|Default|GetNavigationComponent)))
  (if (== (.Lane (Utilities|Struct|BreakMissileData (.MissileData (Utilities|Struct|BreakMissile missile)))) _returnvalue)
    (CallFunction|HandleExplosion))
  (if (<= (Utilities|Array|Length (Class|NavigationComponent|GetIncomingMissiles (Variables|Default|GetNavigationComponent))) 1)
    (Class|BaseCabinet|ChangeState "Inactive")
    (Class|BaseCabinet|BroadcastResult (Utilities|Struct|MakeCabinetResult "Success"))))

(event EventBeginPlay
  (|CallParentFunction)
  (Utilities|FlowControl|Sequence
    (:then_0
      (bind _asbutton_bp (Utilities|Casting|CastToButtonBP (Variables|/Script/Engine.ChildActorComponent|GetChildActor (Variables|Default|GetButtonLeft))))
      (EventDispatchers|BindEventtoOnButtonPressed _asbutton_bp (EventDispatchers|CreateEvent :!event Custom|OnLeftButtonPressed)))
    (:then_1
      (bind _asbutton_bp_2 (Utilities|Casting|CastToButtonBP (Variables|/Script/Engine.ChildActorComponent|GetChildActor (Variables|Default|GetButtonRight))))
      (EventDispatchers|BindEventtoOnButtonPressed _asbutton_bp_2 (EventDispatchers|CreateEvent :!event Custom|OnRightButtonPressed)))
    (:then_2
      (EventDispatchers|BindEventtoMissileImpactEvent (Variables|Default|GetNavigationComponent) (EventDispatchers|CreateEvent :!event Custom|OnMissileImpactEvent)))))

(event EventOnStateChanged
  (params (cabinet :type Base%20Cabinet%20Object%20Reference))
  (bind _maxsalvosiz (Variables|Default|GetMaxSalvoSiz))
  (|CallParentFunction cabinet)
  (bind _returnvalue (Class|BaseCabinet|GetCurrentState cabinet))
  (if (Utilities|Name|Equal(Name) _returnvalue "Active")
    (bind _asnavigation_main_widget_bp (Utilities|Casting|CastToNavigationMainWidgetBP (UserInterface|GetUserWidgetObject (Variables|Default|GetMonitorWidget))))
    (Class|MonitorWidgetInterface|OnActivated _asnavigation_main_widget_bp self)
    (Class|NavigationComponent|ActivateNavigation (Variables|Default|GetNavigationComponent) 0.04 (Variables|Default|GetSalvo%20Size))
    (if (>= (+ (Variables|Default|GetSalvo%20Size) 1.0) _maxsalvosiz)
      (Variables|Default|SetSalvo%20Size _maxsalvosiz)
      (else
        (Variables|Default|SetSalvo%20Size (+ (Variables|Default|GetSalvo%20Size) 1.0))))
    (else
      (bind _asnavigation_main_widget_bp_2 (Utilities|Casting|CastToNavigationMainWidgetBP (UserInterface|GetUserWidgetObject (Variables|Default|GetMonitorWidget))))
      (bind _returnvalue_2 (Class|NavigationComponent|GetCurrentLane (Variables|Default|GetNavigationComponent)))
      (Default|HideWidgets _asnavigation_main_widget_bp_2 _returnvalue_2))))

(event EventTick
  (params (DeltaSeconds :type Float%20%28single-precision%29))
  (|CallParentFunction DeltaSeconds)
  (bind _returnvalue (Class|BaseCabinet|GetCurrentState))
  (if (Utilities|Name|Equal(Name) _returnvalue "Active")
    (CallFunction|ActiveStateUpdate DeltaSeconds)))

(fn ConstructionScript
  (|CallParentFunction))

(fn ActiveStateUpdate
  (params (deltaTime :type Float%20%28single-precision%29))
  (Class|NavigationComponent|UpdateNavigationComponent (Variables|Default|GetNavigationComponent) deltaTime))

(fn HandleExplosion
  (bind _returnvalue (Game|GetPlayerCharacter 0))
  (bind _asonly_one_game_mode (Utilities|Casting|CastToOnlyOneGameMode (Game|GetGameMode)))
  (Default|TakeShipDamage _asonly_one_game_mode 0.1)
  (Utilities|IsValid _returnvalue
    (:Is%20Valid
      (Game|SpawnActorfromClass "/Game/Blueprints/Gameplay/MissileExplosion.MissileExplosion_C" (Math|Transform|MakeTransform (+ (Transformation|GetActorLocation _returnvalue) (* (Math|Random|RandomUnitVector) 5e+03))) "AlwaysSpawn" 0 0))))