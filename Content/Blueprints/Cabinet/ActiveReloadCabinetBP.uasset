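; Active reload minigame cabinet, a child of a cabinet base class, where the player must press a button while an oscillating value is inside a target range.
; While Active, Tick bounces the value between 0 and 1 at a set speed, and activation hands the cabinet to its monitor widget.
; The child button's press event triggers the check, which broadcasts Success or Fail, changes state and plays a sound.
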(event Custom|OnReceiveButtonPress
  ;[1 1 1] Handle receipt of button press by calling OnButtonPressed
  (Variables|Transient|SetButtonPressed true)
  (Utilities|FlowControl|Sequence
    (:then_0
      (bind _returnvalue (Class|BaseCabinet|GetCurrentState))
      (if (not (Utilities|Name|Equal(Name) _returnvalue "Active"))
        (Audio|PlaySoundatLocation "/Game/Audio/Last_bits/Noninteractivebutton.Noninteractivebutton" "0, 0, 0" "0, 0, 0" 0.2 1.0 0.0 0 0 0)))
    (:then_1
      (Class|BaseCabinet|CheckforResult))))

(event EventBeginPlay
  (|CallParentFunction)
  (bind _asbutton_bp (Utilities|Casting|CastToButtonBP (Variables|/Script/Engine.ChildActorComponent|GetChildActor (Variables|Default|GetButton))))
  (EventDispatchers|BindEventtoOnButtonPressed _asbutton_bp (EventDispatchers|CreateEvent :!event Custom|OnReceiveButtonPress)))

(event Collision|EventActorBeginOverlap
  (params (OtherActor :type Actor%20Object%20Reference)))

(event EventTick
  (params (DeltaSeconds :type Float%20%28single-precision%29))
  (bind _returnvalue (Class|BaseCabinet|GetCurrentState))
  (if (Utilities|Name|Equal(Name) _returnvalue "Active")
    (CallFunction|UpdateCurrentValue DeltaSeconds)))

(event EventCheckforResult
  ;[1 1 1] Report a result if button was pressed: Win if it was in range, lose if not
  (|CallParentFunction)
  (bind _returnvalue (Class|BaseCabinet|GetCurrentState))
  (if (and (Utilities|Name|Equal(Name) _returnvalue "Active") (Variables|Transient|GetButtonPressed))
    (if (Math|Float|InRange(Float) (Variables|Transient|GetCurrentValue) (Variables|Setup|GetTargetMin) (Variables|Setup|GetTargetMax))
      (Class|BaseCabinet|BroadcastResult (Utilities|Struct|MakeCabinetResult "Success"))
      (Class|BaseCabinet|ChangeState "Inactive")
      (Audio|PlaySoundatLocation "/Game/Audio/Audio_Assets/minigames/UI_Minigames_Correct_Saw_00.UI_Minigames_Correct_Saw_00" (Transformation|GetWorldLocation (Variables|Default|GetButton_Holder)) "0, 0, 0" 1.0 1.0 0.0 0 0 0)
      (else
        (Class|BaseCabinet|BroadcastResult (Utilities|Struct|MakeCabinetResult "Fail"))
        (Class|BaseCabinet|ChangeState "Fail")
        (Audio|PlaySoundatLocation "/Game/Audio/Audio_Assets/minigames/UI_Minigames_Lose_Square_00.UI_Minigames_Lose_Square_00" (Transformation|GetWorldLocation (Variables|Default|GetButton_Holder)) "0, 0, 0" 1.0 1.0 0.0 0 0 0)))))

(event EventActivateCabinet
  (|CallParentFunction))

(event EventOnStateChanged
  (params (cabinet :type Base%20Cabinet%20Object%20Reference))
  (|CallParentFunction cabinet)
  (bind _returnvalue (Class|BaseCabinet|GetCurrentState))
  (Variables|Transient|SetButtonPressed false)
  (if (Utilities|Name|Equal(Name) _returnvalue "Active")
    (bind _asactive_reload_monitor_widget_bp (Utilities|Casting|CastToActiveReloadMonitorWidgetBP (UserInterface|GetUserWidgetObject (Variables|Default|GetMonitorWidget))))
    (Class|MonitorWidgetInterface|OnActivated _asactive_reload_monitor_widget_bp self)
    (Development|PrintString "Did it")))

(fn ConstructionScript)

(fn UpdateCurrentValue
  (params (deltaTime :type Float%20%28single-precision%29))
  (if (Variables|Transient|GetValueIncreasing)
    (bind _output_get (Variables|Transient|SetCurrentValue (+ (* deltaTime (Variables|Setup|GetSpeed)) (Variables|Transient|GetCurrentValue))))
    (if (>= _output_get 1.0)
      (Variables|Transient|SetCurrentValue 1.0)
      (Variables|Transient|SetValueIncreasing false))
    (else
      (bind _output_get_2 (Variables|Transient|SetCurrentValue (- (Variables|Transient|GetCurrentValue) (* deltaTime (Variables|Setup|GetSpeed)))))
      (if (<= _output_get_2 0.0)
        (Variables|Transient|SetCurrentValue 0.0)
        (Variables|Transient|SetValueIncreasing true)))))