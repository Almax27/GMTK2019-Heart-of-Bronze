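; Base Blueprint for a cabinet actor with a monitor widget and title text that shows its Active, Inactive or Fail state by color.
; The construction script creates a dynamic material instance on the cabinet mesh and applies the current state's color.
; RefreshCabinetMaterial sets the emissive parameter and title text color, rerunning at BeginPlay and whenever the state-changed delegate fires.
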(event Custom|OnStateChanged
  (params (cabinet :type Base%20Cabinet%20Object%20Reference))
  (CallFunction|RefreshCabinetMaterial))

(event EventBeginPlay
  (EventDispatchers|AssignOnCabinetStateChanged (delegate Custom|OnStateChanged))
  (CallFunction|RefreshCabinetMaterial))

(fn ConstructionScript
  (Rendering|Material|CreateDynamicMaterialInstance (Variables|Default|GetCabinet) 1 "/Game/Materials/Master/MessageWarning.MessageWarning" "None" :!class /Script/Engine.PrimitiveComponent)
  (CallFunction|RefreshCabinetMaterial))

(fn GetWidgetComponent
  (return (Variables|Default|GetMonitorWidget)))

(fn RefreshCabinetMaterial
  (bind _returnvalue (Class|BaseCabinet|GetCurrentState))
  (switch name _returnvalue
    (:Active
      (Rendering|Material|SetVectorParameterValueonMaterials (Variables|Default|GetCabinet) "EmissiveColor" (Math|Conversions|ToVector(LinearColor) (Variables|Default|GetActiveColor)))
      (Rendering|Components|TextRender|SetTextRenderColor (Variables|Default|GetTitleText) (Math|Conversions|ToColor(LinearColor) (Variables|Default|GetActiveColor))))
    (:Inactive
      (Rendering|Material|SetVectorParameterValueonMaterials (Variables|Default|GetCabinet) "EmissiveColor" (Math|Conversions|ToVector(LinearColor) (Variables|Default|GetInactiveColor)))
      (Rendering|Components|TextRender|SetTextRenderColor (Variables|Default|GetTitleText) (Math|Conversions|ToColor(LinearColor) (Variables|Default|GetInactiveColor))))
    (:Fail
      (Rendering|Material|SetVectorParameterValueonMaterials (Variables|Default|GetCabinet) "EmissiveColor" (Math|Conversions|ToVector(LinearColor) (Variables|Default|GetFailColor)))
      (Rendering|Components|TextRender|SetTextRenderColor (Variables|Default|GetTitleText) (Math|Conversions|ToColor(LinearColor) (Variables|Default|GetFailColor))))))