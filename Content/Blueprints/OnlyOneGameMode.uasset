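; Game mode for a crewed-ship game, running it from loading screen and intro to win or loss screen.
; It finds room managers, submits intro events, then spawns tactical events and navigation "critical" events on randomized timers once the intro finishes.
; Ship health setters toggle a critical state with music and shield events; zero health loses, full gun charge wins.
; Game events are objects constructed from classes and passed to SubmitGameEvent.
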(event Custom|LoadingFadeInFinished
  ;[1 1 1] Return to title screen
  (Game|OpenLevel(byName) "TitleScreen"))

(event Custom|ReturnToTitleScreen
  (bind _returnvalue (Game|GetPlayerController 0))
  (bind _returnvalue_2 (Game|GetPlayerController 0))
  ;[1 1 1] Return to title screen
  (Utilities|FlowControl|Sequence
    (:then_0
      (Input|SetIgnoreMoveInput _returnvalue_2 true)
      (Input|SetIgnoreLookInput _returnvalue_2 true))
    (:then_1
      (bind _returnvalue_3 (UserInterface|CreateWidget "/Game/Blueprints/UI/LoadingScreenWidget.LoadingScreenWidget_C" _returnvalue))
      (UserInterface|Viewport|AddtoViewport _returnvalue_3 0)
      (Input|SetInputModeUIOnly _returnvalue _returnvalue_3 "DoNotLock")
      (EventDispatchers|BindEventtoFadeinFinished _returnvalue_3 (delegate Custom|LoadingFadeInFinished))
      (Default|StartFadein _returnvalue_3))))

(event Custom|OnShieldsCritical
  (Development|PrintString "Shield is critical" true true "(R=0.000000,G=1.000000,B=0.013595,A=1.000000)")
  (bind _returnvalue (Game|ConstructObjectfromClass "/Game/Blueprints/GameEvents/ShieldCriticalEvent.ShieldCriticalEvent_C" self))
  (Class|GMTKJam2019GameModeBase|SubmitGameEvent _returnvalue))

(event Custom|OnCriticalChanged
  (bind _criticalmusic (Variables|Default|GetCriticalMusic))
  (Utilities|FlowControl|Sequence
    (:then_0
      (if (Variables|Default|GetIsShipCritical)
        (Audio|Components|Audio|FadeIn _criticalmusic 2.0 1.0 0.0 :!class /Script/Engine.AudioComponent)
        (else
          (Audio|Components|Audio|FadeOut _criticalmusic 1.0 0.0 :!class /Script/Engine.AudioComponent))))
    (:then_1
      (Default|CallCriticalStateChanged (Variables|Default|GetIsShipCritical)))))

(event Custom|TriggerNewEvent
  (Utilities|FlowControl|Sequence
    (:then_0
      (bind _returnvalue (Game|ConstructObjectfromClass "/Game/Blueprints/GameEvents/TacticalEvent.TacticalEvent_C" self))
      (Class|GMTKJam2019GameModeBase|SubmitGameEvent _returnvalue))
    (:then_1
      (bind _returnvalue_2 (Utilities|Time|SetTimerbyEvent (EventDispatchers|CreateEvent :!event Custom|TriggerNewEvent) (Math|Random|RandomFloatinRange 1e+01 15.0)))
      (Variables|Transient|SetNextEventTimer _returnvalue_2))))

(event Custom|LoadingFadeOutFinished
  ;[1 1 1] BeginPlay
  (Input|SetInputModeGameOnly (Game|GetPlayerController 0))
  (CallFunction|StartGame))

(event Custom|StartGame
  (bind _array (Utilities|Array|MakeArray "/Game/Blueprints/GameEvents/Intro/IntroStart.IntroStart_C" "/Game/Blueprints/GameEvents/Intro/IntroOpenDoor.IntroOpenDoor_C" "/Game/Blueprints/GameEvents/Intro/IntroNavigation.IntroNavigation_C" "/Game/Blueprints/GameEvents/Intro/IntroTactical.IntroTactical_C" "/Game/Blueprints/GameEvents/Intro/IntroEngineering.IntroEngineering_C" "/Game/Blueprints/GameEvents/Intro/IntroEnd.IntroEnd_C"))
  (for _index (range 0 (Utilities|Array|LastIndex _array))
    (bind _returnvalue (Game|ConstructObjectfromClass (Utilities|Array|Get(acopy) _array _index) self))
    (Class|GMTKJam2019GameModeBase|SubmitGameEvent _returnvalue)))

(event Custom|OnIntroFinished
  (CallFunction|TriggerNewEvent)
  (Utilities|FlowControl|Delay 1e+01)
  (CallFunction|TriggerCriticalEvent))

(event Custom|TriggerCriticalEvent
  (Utilities|FlowControl|Sequence
    (:then_0
      (bind _asgame_event (Utilities|Casting|CastToGameEventClass "/Game/Blueprints/GameEvents/NavigationEvent.NavigationEvent_C"))
      (bind _returnvalue (Game|ConstructObjectfromClass _asgame_event self))
      (Class|GMTKJam2019GameModeBase|SubmitGameEvent _returnvalue))
    (:then_1
      (Utilities|Time|SetTimerbyEvent (delegate Custom|TriggerCriticalEvent) (Math|Random|RandomFloatinRange 6e+01 75.0)))))

(event Custom|EndGame
  (params (Result :type Boolean))
  (bind _returnvalue (Game|GetPlayerController 0))
  (bind _returnvalue_2 (Game|GetPlayerController 0))
  (if (not (Variables|Transient|GetGameEnded))
    (Variables|Transient|SetGameEnded true)
    (Utilities|Time|ClearandInvalidateTimerbyHandle (Variables|Transient|GetNextEventTimer))
    (Input|SetIgnoreMoveInput _returnvalue true)
    (Input|SetIgnoreLookInput _returnvalue true)
    (if Result
      (bind _returnvalue_3 (UserInterface|CreateWidget "/Game/Blueprints/UI/WinScreenWidget.WinScreenWidget_C" _returnvalue_2))
      (UserInterface|Viewport|AddtoViewport _returnvalue_3 0)
      (Input|SetInputModeUIOnly (Game|GetPlayerController 0) _returnvalue_3 "DoNotLock")
      (bind _returnvalue_4 (Game|ConstructObjectfromClass "/Game/Blueprints/GameEvents/EnemyDestroyedEvent.EnemyDestroyedEvent_C" self))
      (Class|GMTKJam2019GameModeBase|SubmitGameEvent _returnvalue_4)
      (else
        (bind _returnvalue_5 (UserInterface|CreateWidget "/Game/Blueprints/UI/LossScreenWidget.LossScreenWidget_C" _returnvalue_2))
        (UserInterface|Viewport|AddtoViewport _returnvalue_5 0)
        (Input|SetInputModeUIOnly (Game|GetPlayerController 0) _returnvalue_5 "DoNotLock")
        (bind _returnvalue_6 (Game|ConstructObjectfromClass "/Game/Blueprints/GameEvents/ShieldFailureEvent.ShieldFailureEvent_C" self))
        (Class|GMTKJam2019GameModeBase|SubmitGameEvent _returnvalue_6)))))

(event Custom|TakeShipDamage
  (params (Damage :type Float%20%28single-precision%29))
  (Development|PrintText (Utilities|Text|FormatText "Ship Damage {0}" Damage))
  (CallFunction|SetShipHealth (- (Variables|Default|GetShipHealth) Damage))
  (if (<= (Variables|Default|GetShipHealth) 0.0)
    (CallFunction|EndGame false)))

(event Custom|OnShieldsRestored
  (Development|PrintString "Shield is restored" true true "(R=0.018294,G=1.000000,B=0.000000,A=1.000000)")
  (bind _returnvalue (Game|ConstructObjectfromClass "/Game/Blueprints/GameEvents/ShieldRestoredEvent.ShieldRestoredEvent_C" self))
  (Class|GMTKJam2019GameModeBase|SubmitGameEvent _returnvalue))

(event EventBeginPlay
  (bind _returnvalue (Game|GetPlayerController 0))
  ;[1 1 1] BeginPlay
  (CallFunction|FindManagers)
  (Variables|Default|SetShipHealth (Variables|Default|GetShipMaxHealth))
  (bind _returnvalue_2 (UserInterface|CreateWidget "/Game/Blueprints/UI/LoadingScreenWidget.LoadingScreenWidget_C" _returnvalue))
  (UserInterface|Viewport|AddtoViewport _returnvalue_2 0)
  (Input|SetInputModeUIOnly _returnvalue _returnvalue_2 "LockAlways")
  (EventDispatchers|BindEventtoFadeOutFinished _returnvalue_2 (delegate Custom|LoadingFadeOutFinished))
  (Default|StartFadeOut _returnvalue_2))

(fn ConstructionScript)

(fn GetCurrentDifficulty
  (if (Utilities|Array|IsValidIndex (Variables|Default|GetDifficultyProgression) (Variables|Transient|GetDIfficultyIndex))
    (return true (Utilities|Array|Get(acopy) (Variables|Default|GetDifficultyProgression) (Variables|Transient|GetDIfficultyIndex)))
    (else
      (return false ""))))

(fn FindManagers
  (Utilities|FlowControl|Sequence
    (:then_0
      (bind _outactors (Actor|GetAllActorsOfClass "/Game/Blueprints/Gameplay/NavigationRoomManager.NavigationRoomManager_C"))
      (if (Utilities|Array|IsValidIndex _outactors)
        (Variables|Transient|SetNavigationRoomManager (Utilities|Array|Get(acopy) _outactors))
        (else
          (Development|PrintString "Failed to find navigation manager" true true "(R=1.000000,G=0.000000,B=0.000000,A=1.000000)" 1e+01))))
    (:then_1
      (bind _outactors_2 (Actor|GetAllActorsOfClass "/Game/Blueprints/Gameplay/TacticalRoomManager.TacticalRoomManager_C"))
      (if (Utilities|Array|IsValidIndex _outactors_2)
        (Variables|Transient|SetTacticalRoomManager (Utilities|Array|Get(acopy) _outactors_2))
        (else
          (Development|PrintString "Failed to find tactical manager" true true "(R=1.000000,G=0.000000,B=0.000000,A=1.000000)" 1e+01))))
    (:then_2
      (bind _outactors_3 (Actor|GetAllActorsOfClass "/Game/Blueprints/Gameplay/EngineeringRoomManager.EngineeringRoomManager_C"))
      (if (Utilities|Array|IsValidIndex _outactors_3)
        (Variables|Transient|SetEngineeringRoomManager (Utilities|Array|Get(acopy) _outactors_3))))
    (:then_3
      (bind _outactors_4 (Actor|GetAllActorsOfClass "/Game/Blueprints/Gameplay/ElevatorManager.ElevatorManager_C"))
      (if (Utilities|Array|IsValidIndex _outactors_4)
        (Variables|Transient|SetElevatorManager (Utilities|Array|Get(acopy) _outactors_4))
        (else
          (Development|PrintString "Failed to find elevator manager" true true "(R=1.000000,G=0.000000,B=0.000000,A=1.000000)" 1e+01))))
    (:then_4
      (bind _outactors_5 (Actor|GetAllActorsOfClass "/Game/Blueprints/Gameplay/CrewQuartersRoomManager.CrewQuartersRoomManager_C"))
      (if (Utilities|Array|IsValidIndex _outactors_5)
        (Variables|Transient|SetCrewQuartersManager (Utilities|Array|Get(acopy) _outactors_5))
        (else
          (Development|PrintString "Failed to find crew quarters manager" true true "(R=1.000000,G=0.000000,B=0.000000,A=1.000000)" 1e+01))))))

(fn SetShipHealth
  (params (NewHealth :type Float%20%28single-precision%29))
  (if (!= (Variables|Default|GetShipHealth) NewHealth)
    (Development|PrintText (Utilities|Text|FormatText "Ship Health: {0} => {1}" (Variables|Default|GetShipHealth) NewHealth))
    (Variables|Default|SetShipHealth NewHealth)
    (Utilities|FlowControl|Sequence
      (:then_0
        (if (<= (Variables|Default|GetShipHealth) (Variables|Default|GetShipCriticalThreshold))
          (if (not (Variables|Default|GetIsShipCritical))
            (Variables|Default|SetIsShipCritical true)
            (CallFunction|OnShieldsCritical)
            (CallFunction|OnCriticalChanged :!label _label))
          (elif (Variables|Default|GetIsShipCritical)
            (Variables|Default|SetIsShipCritical false)
            (CallFunction|OnShieldsRestored)
            (goto _label))))
      (:then_1
        (Default|CallShipHealthChanged (Variables|Default|GetShipHealth))))))

(fn SetGunCharge
  (params (NewValue :type Float%20%28single-precision%29))
  (if (!= (Variables|Default|GetGunCharge) NewValue)
    (Development|PrintText (Utilities|Text|FormatText "Gun Charge: {0} => {1}" (Variables|Default|GetGunCharge) NewValue))
    (bind _output_get (Variables|Default|SetGunCharge NewValue))
    (Default|CallGunChargeChanged _output_get)
    (if (>= NewValue 1.0)
      (CallFunction|EndGame true))))

(fn AddGunCharge
  (params (Delta :type Float%20%28single-precision%29))
  (CallFunction|SetGunCharge (+ Delta (Variables|Default|GetGunCharge))))

(fn ResetShipHealth
  (CallFunction|SetShipHealth (Variables|Default|GetShipMaxHealth)))